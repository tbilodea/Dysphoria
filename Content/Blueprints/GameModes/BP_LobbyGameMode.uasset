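; Lobby game mode for a Steam multiplayer session that tracks connected players, game settings, kicks and the loading screen.
; PostLogin records the player, pulls server name and max players from the Steam game instance, and sets up their lobby menu; SpawnPlayer is an empty stub.
; EveryoneUpdate, run on login and logout, rebuilds player info and pushes it with counts and settings to every lobby controller through reference-getter messages.
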(event Custom|SpawnPlayer
  (params (PlayerController :type Player%20Controller%20Object%20Reference))
  ;[1 1 1] Initial setup that starts each time a new player connects - the lobby should update for each connected player
)

(event Custom|StartLoadingScreen
  ;[1 1 1] Starts Loading screen for every Connected player
  (for _array_element (Variables|Default|GetPlayers)
    (bind _lobbypc (Class|BPIMenuPlayerController|LobbyPCRef(Message) _array_element))
    (Default|ShowLoadingScreen _lobbypc)))

(event Custom|AddToKickList
  ;[1 1 1] Add Connected players to kick list
  (bind _lobbypc (Class|BPIMenuPlayerController|LobbyPCRef(Message) (Game|GetPlayerController 0)))
  (Default|AddPlayertoKickWindow _lobbypc))

(event Custom|UpdateGameSettings
  (params (Difficulty :type Integer) (StandardMode :type Boolean))
  ;[1 1 1] Server made game settings changes, sets variables to update screens
  (Variables|Default|SetDifficultyPercent Difficulty)
  (Variables|Default|SetGameTypeStandard StandardMode))

(event Custom|PlayerKicked
  (params (PlayerId :type Integer))
  ;[1 1 1] Kick selected player from session
  (bind _lobbypc (Class|BPIMenuPlayerController|LobbyPCRef(Message) (Utilities|Array|Get(acopy) (Variables|Default|GetPlayers) PlayerId)))
  (Default|Kicked _lobbypc))

(event Custom|EveryoneUpdate
  (bind _players (Variables|Default|GetPlayers))
  ;[1 1 1] Updates All Player Lobby Widget information when called
  (bind _output_get (Variables|Default|SetCurrentPlayers (Utilities|Array|Length (Variables|Default|GetPlayers))))
  (if (> _output_get 0)
    (Utilities|Array|Clear (Variables|Default|GetConnectedPlayerInfo))
    (for _array_element _players
      (bind _lobbypc (Class|BPIMenuPlayerController|LobbyPCRef(Message) _array_element))
      (Utilities|Array|AddUnique (Variables|Default|GetConnectedPlayerInfo) (Variables|/Game/Blueprints/PlayerControllers/BP_LobbyPC.BP_LobbyPC_C|GetPlayerSettings _lobbypc))
      (Default|UpdateNumberOfPlayers _lobbypc (Variables|Default|GetCurrentPlayers) (Variables|Default|GetMaxPlayers))
      (Default|UpdateGameSettings _lobbypc (Variables|Default|GetDifficultyPercent) (Variables|Default|GetGameTypeStandard)))
    (for _array_element_2 _players
      (bind _lobbypc_2 (Class|BPIMenuPlayerController|LobbyPCRef(Message) _array_element_2))
      (Default|AddPlayerInfo _lobbypc_2 (Variables|Default|GetConnectedPlayerInfo))
      (CallFunction|AddtoKickList))
    (bind _array_element_3 (Utilities|Array|ForEachLoopwithBreak (Variables|Default|GetConnectedPlayerInfo)))))

(event Custom|CannotStartGame
  ;[1 1 1] Updates All Player Lobby Widget information when called
  (Utilities|Array|ForEachLoopwithBreak (Variables|Default|GetConnectedPlayerInfo)) ; enters at Break
)

(event EventOnLogout
  (params (ExitingController :type Controller%20Object%20Reference))
  (bind _players (Variables|Default|GetPlayers))
  ;[1 1 1] Removes the player  information and updates everyone when someone logs out
  (bind (_array_element _array_index) (Utilities|Array|ForEachLoopwithBreak _players :!label _label)
    (:LoopBody
      (if (== _array_element ExitingController)
        (goto _label Break)))
    (:Completed
      (Class|BPIMenuPlayerController|LobbyPCRef(Message) (Utilities|Array|Get(acopy) _players _array_index))
      (Utilities|Array|RemoveIndex (Variables|Default|GetConnectedPlayerInfo) _array_index)
      (Utilities|Array|RemoveIndex (Variables|Default|GetPlayers) _array_index)
      (CallFunction|EveryoneUpdate))))

(event EventPostLogin
  (params (NewPlayer :type Player%20Controller%20Object%20Reference))
  ;[1 1 1] Initial setup that starts each time a new player connects - the lobby should update for each connected player
  (bind _output_get (Variables|Default|SetConnectedPlayer NewPlayer))
  (Utilities|Array|AddUnique (Variables|Default|GetPlayers) _output_get)
  (bind _outactors (Actor|GetAllActorsOfClass "/Script/Engine.PlayerStart"))
  (Variables|Default|SetSpawnPoints _outactors)
  (bind _newparam (Class|BPIGameInstance|SteamGameInstanceRef(Message) (Game|GetGameInstance)))
  (Variables|Default|SetServerName (Variables|/Game/Blueprints/BP_SteamGameInstance.BP_SteamGameInstance_C|GetServerName _newparam))
  (Variables|Default|SetMaxPlayers (Variables|/Game/Blueprints/BP_SteamGameInstance.BP_SteamGameInstance_C|GetMaxPlayers _newparam))
  (bind _lobbypc (Class|BPIMenuPlayerController|LobbyPCRef(Message) (Variables|Default|GetConnectedPlayer)))
  (Default|InitialSetup _lobbypc)
  (Default|SetupLobbyMenu _lobbypc (Utilities|Text|ToText(String) (Variables|Default|GetServerName)))
  (CallFunction|EveryoneUpdate)
  (CallFunction|SpawnPlayer (Variables|Default|GetConnectedPlayer)))

(fn ConstructionScript)

(fn LobbyGMRef
  (return self))