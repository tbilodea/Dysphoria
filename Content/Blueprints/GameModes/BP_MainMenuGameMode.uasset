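; Main menu game mode that sets up the lobby for each player who logs in.
; PostLogin records the player, gathers PlayerStart actors and reads server name and max players from the Steam game instance through a message call.
; It then tells the player's menu controller to run initial setup, build the lobby menu and show default map settings.
; The closing SpawnPlayer call is an empty stub, so the gathered spawn points are unused here.
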(event Custom|SpawnPlayer
  (params (PlayerController :type Player%20Controller%20Object%20Reference)))

(event EventPostLogin
  (params (NewPlayer :type Player%20Controller%20Object%20Reference))
  (bind _output_get (Variables|Default|SetConnectedPlayer NewPlayer))
  (Utilities|Array|AddUnique (Variables|Default|GetPlayers) _output_get)
  (bind _outactors (Actor|GetAllActorsOfClass "/Script/Engine.PlayerStart"))
  (Variables|Default|SetSpawnPoints _outactors)
  (bind _newparam (Class|BPIGameInstance|SteamGameInstanceRef(Message) (Game|GetGameInstance)))
  (Variables|Default|SetServerName (Variables|/Game/Blueprints/BP_SteamGameInstance.BP_SteamGameInstance_C|GetServerName _newparam))
  (Variables|Default|SetMaxPlayers (Variables|/Game/Blueprints/BP_SteamGameInstance.BP_SteamGameInstance_C|GetMaxPlayers _newparam))
  (bind _mainmenupc (Class|BPIMenuPlayerController|MenuPCRef(Message) (Variables|Default|GetConnectedPlayer)))
  (Default|InitialSetup _mainmenupc)
  (Default|SetupLobbyMenu _mainmenupc (Utilities|Text|ToText(String) (Variables|Default|GetServerName)))
  (Default|UpdateLobbySettings _mainmenupc (Variables|Default|GetDefaultMapName) (Variables|Default|GetDefaultMapTime) (Variables|Default|GetDefaultMapImage))
  (CallFunction|SpawnPlayer (Variables|Default|GetConnectedPlayer)))

(fn ConstructionScript)