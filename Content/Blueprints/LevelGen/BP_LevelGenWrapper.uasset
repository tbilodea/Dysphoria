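; BP_LevelGenWrapper is an actor that builds and lays out a room-grid level when play begins.
; It constructs a LevelGenerator object, generates the level and caches the boss room, entrance room and grid dimensions.
; It then spawns a BP_BuildRoom at each spaced row and column cell and passes in that cell's room data.
; Cells matching the entrance or boss room are flagged as such, and missing room data prints a failure message.
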(event Custom|GetBossRoom
  (Variables|Default|SetBossRoom (Class|LevelGenerator|GetBossRoom (Variables|Default|GetLevelGenerator))))

(event Custom|GetEntranceRoom
  (Variables|Default|SetEntrance%20Room (Class|LevelGenerator|GetEntrance (Variables|Default|GetLevelGenerator))))

(event EventBeginPlay
  (bind _spacingbetweenrooms (Variables|Default|GetSpacingBetweenRooms))
  (bind _bossroom (Variables|Default|GetBossRoom))
  (bind _entrance_room (Variables|Default|GetEntrance%20Room))
  ;[1 1 1] Builds and lays out level
  (bind _returnvalue (Game|ConstructObjectfromClass "/Script/Dysphoria.LevelGenerator" self))
  (bind _output_get (Variables|Default|SetLevelGenerator _returnvalue))
  (Class|LevelGenerator|GenerateLevel _output_get)
  (CallFunction|GetBossRoom)
  (CallFunction|GetEntranceRoom)
  (bind _output_get_2 (Variables|Default|SetRows (Class|LevelGenerator|GetRows _output_get)))
  (bind _output_get_3 (Variables|Default|SetCols (Class|LevelGenerator|GetCols _output_get)))
  (bind _intarray (CallFunction|CreateIntArray _output_get_2))
  (bind _output_get_4 (Variables|Default|SetRowArray _intarray))
  (bind _intarray_2 (CallFunction|CreateIntArray _output_get_3))
  (bind _output_get_5 (Variables|Default|SetColArray _intarray_2))
  (for _array_element _output_get_4
    (for _array_element_2 _output_get_5
      (bind _returnvalue_2 (Game|SpawnActorfromClass "/Game/Test/BP_BuildRoom.BP_BuildRoom_C" (Math|Transform|MakeTransform (Math|Vector|MakeVector (* _array_element _spacingbetweenrooms) (* _array_element_2 _spacingbetweenrooms) 0.0)) "AlwaysSpawn" 0 0))
      (if (Utilities|IsValid (Class|LevelGenerator|GetRoom (Variables|Default|GetLevelGenerator) _array_element _array_element_2))
        (Default|SetRoomData _returnvalue_2 (Class|LevelGenerator|GetRoom (Variables|Default|GetLevelGenerator) _array_element _array_element_2) _array_element _array_element_2)
        (if (and (== _array_element (Class|RowCol|GetRow _entrance_room)) (== _array_element_2 (Class|RowCol|GetCol _entrance_room)))
          (Default|SetasEntranceRoom _returnvalue_2)
          (elif (and (== _array_element (Class|RowCol|GetRow _bossroom)) (== _array_element_2 (Class|RowCol|GetCol _bossroom)))
            (Default|SetasBossRoom _returnvalue_2)))
        (else
          (Development|PrintString "Failed to find the room data"))))))

(event Collision|EventActorBeginOverlap
  (params (OtherActor :type Actor%20Object%20Reference)))

(event EventTick
  (params (DeltaSeconds :type Float%20%28single-precision%29)))

(fn ConstructionScript)

(fn CreateIntArray
  (params (MaxValue :type Integer))
  (bind _newinttoadd (LocalVariables|GetNewIntToAdd))
  ;[1 1 1] Create a new int array up to the max (not including)
  (while (< (LocalVariables|GetNewIntToAdd) MaxValue)
    (Utilities|Array|Add (LocalVariables|GetIntArrayToReturn) _newinttoadd)
    (Math|Integer|IncrementInt _newinttoadd))
  (return (LocalVariables|GetIntArrayToReturn)))