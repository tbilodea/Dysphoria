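; BP_LobbyPC is the lobby player controller that manages each player's lobby menu and session exit.
; It creates the LobbyMenu widget with the server name, then forwards player count, game settings, player list and host kick-window updates to it.
; It stores player settings and swaps the menu for a loading screen when requested.
; Being kicked opens MainMenu and destroys the session, which EndPlay also does.
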(event Custom|InitialSetup)

(event Custom|SetupLobbyMenu
  (params (ServerName :type Text))
  (Variables|Default|SetbShowMouseCursor true)
  (bind _returnvalue (UserInterface|CreateWidget "/Game/Blueprints/Lobby/LobbyMenu.LobbyMenu_C" 0 ServerName))
  (bind _output_get (Variables|Default|SetLobbyWidget _returnvalue))
  (UserInterface|Viewport|AddtoViewport _output_get 0)
  (Input|SetInputModeGameandUI self (Variables|Default|GetLobbyWidget) "DoNotLock" true))

(event Custom|AddPlayerInfo
  (params (PlayersInfo :type Array%20of%20S%20Player%20Info%20Structures))
  ;[1 1 1] Update the player list widget
  (Variables|Default|SetAllConnectedPlayers PlayersInfo)
  (bind _lobbywidget (Variables|Default|GetLobbyWidget)
    (:then
      (Default|ClearPlayerList _lobbywidget)
      (for _array_element (Variables|Default|GetAllConnectedPlayers)
        (Default|UpdatePlayerWindow (Variables|Default|GetLobbyWidget) _array_element)))
    (:else)))

(event Custom|CallUpdate
  (params (Settings :type S%20Player%20Info%20Structure) (ChangedStatus :type Boolean))
  (Variables|Default|SetPlayerSettings Settings))

(event Custom|ShowLoadingScreen
  (Widget|RemovefromParent (Variables|Default|GetLobbyWidget))
  (bind _returnvalue (UserInterface|CreateWidget "/Game/Blueprints/Widget/LoadingScreen.LoadingScreen_C" self))
  (UserInterface|Viewport|AddtoViewport _returnvalue 0))

(event Custom|Kicked
  ;[1 1 1] Player Kicked or Server Disconnects
  (Game|OpenLevel(byName) "MainMenu")
  (|DestroySession self))

(event Custom|UpdateGameSettings
  (params (Difficulty :type Integer) (StandardMode :type Boolean))
  ;[1 1 1] Updates the lobby game settings
  (Default|UpdateGameSettings (Variables|Default|GetLobbyWidget) Difficulty StandardMode))

(event Custom|UpdateNumberOfPlayers
  (params (CurrentPlayers :type Integer) (MaxPlayers :type Integer))
  (Default|UpdatePlayersDisplay (Variables|Default|GetLobbyWidget) (Utilities|Text|FormatText "{CurrentPlayers} of {MaxPlayers}" (Utilities|Text|ToText(Integer) CurrentPlayers) (Utilities|Text|ToText(Integer) MaxPlayers))))

(event Custom|AddPlayerToKickWindow
  ;[1 1 1] Updates host kick window
  (bind _lobbywidget (Variables|Default|GetLobbyWidget)
    (:then
      (Default|AddPlayertoKickWindow _lobbywidget))
    (:else)))

(event EventEndPlay
  (params (EndPlayReason :type EEndPlayReason%20Enum :default "Destroyed"))
  ;[1 1 1] Player Kicked or Server Disconnects
  (|DestroySession self))

(fn ConstructionScript)

(fn LobbyPCRef
  (return self))