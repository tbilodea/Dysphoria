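; Game instance that drives the multiplayer front end: menus, loading screen, session hosting, joining and destruction, and error popups.
; Menu events create and cache their widgets before adding them to the viewport, except the server menu, which is rebuilt on every call.
; Hosting creates a session and opens the Lobby as a listen server.
; Host or join failures and network or travel errors feed one reused error window, with most network failures reported as lost connection.
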(event EventShowMainMenu
  (bind _returnvalue (Game|GetPlayerController 0))
  ;[1 1 1] Launch Main Menu and Enable Mouse Cursor
  (Variables|Default|GetMainMenu
    (:then
      _)
    (:else
      (bind _returnvalue_2 (UserInterface|CreateWidget "/Game/Blueprints/Menus/MainMenu.MainMenu_C" _returnvalue))
      (bind _output_get (Variables|Default|SetMainMenu _returnvalue_2))))
  (UserInterface|Viewport|AddtoViewport _output_get 0)
  (Variables|/Script/Engine.PlayerController|SetbShowMouseCursor _returnvalue true))

(event EventHandleNetworkError
  (params (FailureType :type ENetworkFailure%20Enum :default "NetDriverAlreadyExists") (bIsServer :type Boolean))
  ;[1 1 1] Show Network Error to player
  (if bIsServer
    _
    (else
      _))
  (Utilities|ErrorMessage (CallFunction|NetworkErrortoString FailureType)))

(event EventDestroySession
  (params (PlayerController :type Player%20Controller%20Object%20Reference))
  ;[1 1 1] Destroys the Session when Called
  (|DestroySession PlayerController))

(event EventHandleTravelError
  (params (FailureType :type ETravelFailure%20Enum :default "NoLevel"))
  ;[1 1 1] Show Travel Error to player
  (Utilities|ErrorMessage (CallFunction|TravelErrortoString FailureType)))

(event EventShowHostMenu
  ;[1 1 1] Show Host Menu
  (Variables|Default|GetHostMenu
    (:then
      _)
    (:else
      (bind _returnvalue (UserInterface|CreateWidget "/Game/Blueprints/Menus/HostMenu.HostMenu_C" (Game|GetPlayerController 0)))
      (bind _output_get (Variables|Default|SetHostMenu _returnvalue))))
  (UserInterface|Viewport|AddtoViewport _output_get 0))

(event EventShowServerMenu
  ;[1 1 1] Always generate a new Server Menu
  (bind _returnvalue (UserInterface|CreateWidget "/Game/Blueprints/Menus/ServerMenu.ServerMenu_C" (Game|GetPlayerController 0)))
  (UserInterface|Viewport|AddtoViewport _returnvalue 0))

(event EventShowOptionsMenu
  ;[1 1 1] Show Options Menu
  (Variables|Default|GetOptionsMenu
    (:then
      _)
    (:else
      (bind _returnvalue (UserInterface|CreateWidget "/Game/Blueprints/Menus/OptionsMenu.OptionsMenu_C" (Game|GetPlayerController 0)))
      (bind _output_get (Variables|Default|SetOptionsMenu _returnvalue))))
  (UserInterface|Viewport|AddtoViewport _output_get 0))

(event EventShowLoadingScreen
  ;[1 1 1] Shows Loading Screen
  (Variables|Default|GetLoadingScreen
    (:then
      _)
    (:else
      (bind _returnvalue (UserInterface|CreateWidget "/Game/Blueprints/Widget/LoadingScreen.LoadingScreen_C" (Game|GetPlayerController 0)))
      (bind _output_get (Variables|Default|SetLoadingScreen _returnvalue))))
  (UserInterface|Viewport|AddtoViewport _output_get 0))

(event EventLaunchLobby
  (params (NumberOfPlayers :type Integer) (EnableLan :type Boolean) (ServerName :type String))
  ;[1 1 1] Launch the Lobby Level
  (bind _output_get (Variables|Default|SetMaxPlayers NumberOfPlayers))
  (Variables|Default|SetServerName ServerName)
  (CallFunction|ShowLoadingScreen)
  (|Session (Game|GetPlayerController 0) _output_get EnableLan
    (:OnSuccess
      (Game|OpenLevel(byName) "Lobby" true "listen"))
    (:OnFailure
      (Utilities|ErrorMessage "Failed to launch lobby, please try again."))))

(event EventJoinServer
  (params (SessionToJoin :type Blueprint%20Session%20Result%20Structure))
  ;[1 1 1] Join the Server
  (CallFunction|ShowLoadingScreen)
  (|JoinSession (Game|GetPlayerController 0) SessionToJoin
    (:OnFailure
      (Utilities|ErrorMessage "Failed to join server, please try again."))))

(fn NetworkErrortoString
  (params (NetworkFailure :type ENetworkFailure%20Enum :default "NetDriverAlreadyExists"))
  (switch Utilities|FlowControl|Switch|SwitchonENetworkFailure NetworkFailure
    (:NetDriverAlreadyExists
      (LocalVariables|SetErrorString "Error: Lost Connection to Host" :!label _label))
    (:NetDriverCreateFailure
      (goto _label))
    (:NetDriverListenFailure
      (goto _label))
    (:ConnectionLost
      (goto _label))
    (:ConnectionTimeout
      (LocalVariables|SetErrorString "Error: Connection Timed Out"))
    (:FailureReceived
      (goto _label))
    (:OutdatedClient
      (goto _label))
    (:OutdatedServer
      (goto _label))
    (:PendingConnectionFailure
      (goto _label)))
  (return (LocalVariables|GetErrorString)))

(fn TravelErrortoString
  (params (FailureType :type ETravelFailure%20Enum :default "NoLevel"))
  (return (Utilities|String|Append "Error: Failed to Travel -- " (Utilities|String|EnumtoString FailureType))))

(fn SteamGameInstanceRef
  (return self))