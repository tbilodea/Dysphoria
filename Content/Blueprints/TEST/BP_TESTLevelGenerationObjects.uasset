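; Test Blueprint for grid-based level generation, exercising the LevelData and LevelLayout objects through their TESTBP functions.
; BeginPlay constructs both objects, links them and runs the LevelLayout tests; the LevelData tests are present but disconnected.
; Most tests first call ReinitLevelData to rebuild a 5x5 map with two known door connections.
; Checks compare results to hardcoded expectations, and PassFail prints each outcome on screen.
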(event Custom|Reinit%20LevelData
  (bind _leveldata (Variables|Default|GetLevelData))
  ;[1 1 1] Reinitialized Level connections, default adds a door between [0,0] and [0,1] as well as [4,4] and [3,4]
  (Class|LevelData|InitializeLevelDataMap _leveldata 5 5)
  (Class|LevelData|TESTBPAddDoorsBetween _leveldata 0 0 0 1)
  (Class|LevelData|TESTBPAddDoorsBetween _leveldata 4 4 3 4)
  (Development|PrintString "Reinit Level Data"))

(event EventBeginPlay
  ;[1 1 1] Initialize Level Data and Level Layout
  (bind _returnvalue (Game|ConstructObjectfromClass "/Script/Dysphoria.LevelData" self))
  (bind _output_get (Variables|Default|SetLevelData _returnvalue))
  (bind _returnvalue_2 (Game|ConstructObjectfromClass "/Script/Dysphoria.LevelLayout" self))
  (bind _output_get_2 (Variables|Default|SetLevelLayout _returnvalue_2))
  (Class|LevelLayout|TESTBPSetLevelData _output_get_2 _output_get)
  ;[1 1 1] Level Layout Tests
  (CallFunction|TestGetRoomLocationinDirection)
  (CallFunction|TestGetNeighborstoAttachto)
  (CallFunction|TestEnsureRandomLocationinBounds))

(event Collision|EventActorBeginOverlap
  (params (OtherActor :type Actor%20Object%20Reference)))

(event EventTick
  (params (DeltaSeconds :type Float%20%28single-precision%29)))

(fn ConstructionScript)

(fn TestDirectionsWithoutDoors
  (CallFunction|ReinitLevelData)
  ;[1 1 1] Connected to EAST, in Corner (W, S) returns N
  (bind _returnvalue (Class|LevelData|TESTBPGetDirectionsWithoutDoors (Variables|Default|GetLevelData)))
  (LocalVariables|SetTest1 _returnvalue)
  (CallFunction|PassFail "DirectionsWithoutDoors #1" (Utilities|Array|ContainsItem _returnvalue 0))
  ;[1 1 1] Has 1 Direction, WEST (Connected S, Corner of map)
  (bind _returnvalue_2 (Class|LevelData|TESTBPGetDirectionsWithoutDoors (Variables|Default|GetLevelData) 4 4))
  (CallFunction|PassFail "DirectionsWithoutDoors #2" (Utilities|Array|ContainsItem _returnvalue_2 3))
  ;[1 1 1] Has 2 Directions, SOUTH and WEST - Connected to NORTH and on the Right Edge of map
  (bind _returnvalue_3 (Class|LevelData|TESTBPGetDirectionsWithoutDoors (Variables|Default|GetLevelData) 3 4))
  (CallFunction|PassFail "DirectionsWithoutDoors #3" (and (Utilities|Array|ContainsItem _returnvalue_3 2) (Utilities|Array|ContainsItem _returnvalue_3 3)))
  ;[1 1 1] Has all directions
  (bind _returnvalue_4 (Class|LevelData|TESTBPGetDirectionsWithoutDoors (Variables|Default|GetLevelData) 2 2))
  (CallFunction|PassFail "DirectionsWithoutDoors #4" (== (Utilities|Array|Length _returnvalue_4) 4)))

(fn PassFail
  (params (NameOfFunction :type String) (Pass :type Boolean) (FailText :type String))
  (Development|PrintString (Utilities|String|Append NameOfFunction "\" [ \"" (Utilities|String|ToString(Boolean) Pass) "\" ] \"" FailText) true true "(R=0.000000,G=0.660000,B=1.000000,A=1.000000)" 15.0))

(fn TestGetNeighborsOf
  (CallFunction|ReinitLevelData)
  (bind _returnvalue (Class|LevelData|TESTBPGetNeighborsOf (Variables|Default|GetLevelData)))
  (CallFunction|PassFail "GetNeighborsOf Test #1" (== (Utilities|Array|Length _returnvalue) 4))
  (bind _returnvalue_2 (Class|LevelData|TESTBPGetNeighborsOf (Variables|Default|GetLevelData) 2 2))
  (CallFunction|PassFail "GetNeighborsOf Test #2" (== (Utilities|Array|Length _returnvalue_2) 8)))

(fn TestGetNeighborswithDoors
  (CallFunction|ReinitLevelData)
  (bind _returnvalue (Class|LevelData|TESTBPGetNeighborswithDoors (Variables|Default|GetLevelData)))
  (LocalVariables|SetTestSuccess true)
  (for (_array_element _array_index) _returnvalue
    (if (not (and (== _array_element 0) (== _array_index 0)))
      (if (not (and (== _array_element 1) (== _array_index 1)))
        (LocalVariables|SetTestSuccess false))))
  (CallFunction|PassFail "Get Neighbors With Doors Test #1" (LocalVariables|GetTestSuccess)))

(fn TestGetNeighborstoAttachto
  (CallFunction|ReinitLevelData)
  (bind _arrayhasrooms (CallFunction|CheckRoomLocationIs (Class|LevelLayout|TESTBPGetNeighbortoAttachto (Variables|Default|GetLevelLayout) 1 1) 0 1))
  (CallFunction|PassFail "Rooms to attach to #1" _arrayhasrooms)
  (bind _arrayhasrooms_2 (CallFunction|CheckRoomLocationIs (Class|LevelLayout|TESTBPGetNeighbortoAttachto (Variables|Default|GetLevelLayout) 3 3) 3 4))
  (CallFunction|PassFail "Rooms to attach to #2" _arrayhasrooms_2))

(fn TestGetRoomLocationinDirection
  (bind _arrayhasrooms (CallFunction|CheckRoomLocationIs (Class|LevelLayout|TESTBPGetRoomLocationinDirection (Variables|Default|GetLevelLayout) 0 0 "NORTH") 1))
  (CallFunction|PassFail "Get Room Location in Direction" _arrayhasrooms))

(fn TestEnsureRandomLocationinBounds
  (LocalVariables|SetSuccess true)
  (bind _array_element (Utilities|Array|ForEachLoopwithBreak (Class|LevelLayout|TESTBPGetRandomDirection (Variables|Default|GetLevelLayout)) :!label _label)
    (:LoopBody
      (if (> _array_element 4)
        (LocalVariables|SetExtraInfo (Utilities|String|Append (Utilities|String|ToString(Integer) _array_element) " is over the max row/col of 4"))
        (LocalVariables|SetSuccess false)
        (goto _label Break)))
    (:Completed
      (CallFunction|PassFail "GetRandomLocation #1" (LocalVariables|GetSuccess) (LocalVariables|GetExtraInfo)))))

(fn CheckRoomLocationIs
  (params (NewParam :type Array%20of%20Integers) (Row :type Integer) (Col :type Integer))
  (LocalVariables|SetSuccessfulTest true)
  (for (_array_element _array_index) NewParam
    (if (not (and (== _array_index 0) (== _array_element Row)))
      (if (not (and (== _array_index 1) (== _array_element Col)))
        (LocalVariables|SetSuccessfulTest false))))
  (return (LocalVariables|GetSuccessfulTest)))