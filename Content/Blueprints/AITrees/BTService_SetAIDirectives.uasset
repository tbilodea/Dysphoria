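; Behavior tree service that copies an AI entity's current directive into its blackboard.
; On each tick it casts the controlled pawn to BaseAIEntity, fetches its AI directive and writes the directive enum, focused player and focused entity to blackboard keys.
; Debug prints report a missing directive, a pawn of the wrong type, or a value after a successful update.
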(event EventReceiveTickAI
  (params (OwnerController :type AI%20Controller%20Object%20Reference) (ControlledPawn :type Pawn%20Object%20Reference) (DeltaSeconds :type Float%20%28single-precision%29))
  (bind _asbase_aientity (Utilities|Casting|CastToBaseAIEntity ControlledPawn)
    (:then
      (bind _returnvalue (Class|AIEntity|GetAIDirective _asbase_aientity))
      (if (== _returnvalue 0)
        (Development|PrintString "AIDirective doesn't exist")
        (else
          (Class|BTFunctionLibrary|SetBlackboardValueasEnum (Variables|Default|GetDirective) (Variables|/Script/Dysphoria.SwarmDirective|GetDirective _returnvalue))
          (Class|BTFunctionLibrary|SetBlackboardValueasObject (Variables|Default|GetPlayer) (Variables|/Script/Dysphoria.SwarmDirective|GetFocusedPlayer _returnvalue))
          (Class|BTFunctionLibrary|SetBlackboardValueasObject (Variables|Default|GetAIEntity) (Variables|/Script/Dysphoria.SwarmDirective|GetFocusedEntity _returnvalue))
          (Development|PrintString (Utilities|String|ToString(Object) 0)))))
    (:CastFailed
      (Development|PrintString "This ai isn't a base enemy"))))