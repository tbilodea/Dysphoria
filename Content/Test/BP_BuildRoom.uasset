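; BP_BuildRoom is a test room actor that configures its meshes from room data it is given.
; SetRoomData stores the data and swaps each listed door direction's static mesh component (north, east, south, west) to the door mesh.
; SetAsBossRoom and SetAsEntranceRoom both apply the same highlight material to the floor, and leftover debug material and print nodes are disconnected.
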(event Custom|Set%20Room%20Data
  (params (NewRoomData :type Room%20Data%20Object%20Reference) (Row :type Integer) (Col :type Integer))
  (bind _doormesh (Variables|Default|GetDoorMesh))
  (bind _output_get (Variables|Default|SetRoomData NewRoomData))
  ;[1 1 1] Turns the right doors on/off
  (if (and (== Row Col) (== Col 0))
    _
    (else
      _))
  (bind _result (Utilities|Set|ToArray (Class|RoomData|GetDoors _output_get)))
  (for _array_element _result
    (Variables|Default|SetDirectionsStrs (Utilities|String|Append (Variables|Default|GetDirectionsStrs) " " (Utilities|String|EnumtoString _array_element)))
    (switch Utilities|FlowControl|Switch|SwitchonDirection _array_element
      (:NORTH
        (Components|StaticMesh|SetStaticMesh (Variables|Default|GetDoorNorth) _doormesh))
      (:EAST
        (Components|StaticMesh|SetStaticMesh (Variables|Default|GetDoorEast) _doormesh))
      (:SOUTH
        (Components|StaticMesh|SetStaticMesh (Variables|Default|GetDoorSouth) _doormesh))
      (:WEST
        (Components|StaticMesh|SetStaticMesh (Variables|Default|GetDoorWest) _doormesh)))))

(event Custom|SetAsEntranceRoom
  (Rendering|Material|SetMaterial (Variables|Default|GetFloor) 0 "/Game/Examples/FirstPerson/Meshes/FirstPersonProjectileMaterial.FirstPersonProjectileMaterial"))

(event Custom|SetAsBossRoom
  (Rendering|Material|SetMaterial (Variables|Default|GetFloor) 0 "/Game/Examples/FirstPerson/Meshes/FirstPersonProjectileMaterial.FirstPersonProjectileMaterial"))

(event EventBeginPlay)

(event Collision|EventActorBeginOverlap
  (params (OtherActor :type Actor%20Object%20Reference)))

(event EventTick
  (params (DeltaSeconds :type Float%20%28single-precision%29)))

(fn ConstructionScript)